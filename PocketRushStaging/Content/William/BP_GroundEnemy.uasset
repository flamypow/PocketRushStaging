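; Ground enemy Blueprint that fires projectiles at the player character when pawn sensing spots it.
; Each sighting calls CheckPlayer, then turns ShootPosition toward the seen BP_PocketRushCharacter with a look-at rotation.
; A Delay derived from AttackSpeed paces firing, after which Shoot plays the robot attack montage and spawns ProjectileRef at ShootPosition's transform.
; BeginPlay and construction defer to the parent class.
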(event `self.PawnSensing.OnSeePawn`
  (params (Pawn :type "Pawn Object Reference"))
  (`self.CheckPlayer` Pawn)
  (`self.Set Shoot Rotation` Pawn)
  (`KismetSystemLibrary.Delay` (/ 1.0 (`self.AttackSpeed`)))
  (`self.Shoot`))

(event `self.ReceiveBeginPlay`
  (`parent.ReceiveBeginPlay`))

(fn `Set Shoot Rotation`
  (params (PlayerObj :type "Object Object Reference"))
  (bind _asbp_pocket_rush_character (cast `/Game/KillianContent/BP_PocketRushCharacter` PlayerObj))
  (`SceneComponent.K2_SetWorldRotation` (`self.ShootPosition`) (`KismetMathLibrary.FindRelativeLookAtRotation` (`KismetMathLibrary.Conv_VectorToTransform` (`SceneComponent.K2_GetComponentLocation` (`self.ShootPosition`))) (`self.K2_GetActorLocation` _asbp_pocket_rush_character)) false false))

(fn `Shoot`
  (`self.PlayAnimMontage` "/Game/William/AM_EnemyRobot_Attack.AM_EnemyRobot_Attack")
  (`|SpawnActorFromClass` (`self.ProjectileRef`) (`SceneComponent.K2_GetComponentToWorld` (`self.ShootPosition`)) "Undefined" "MultiplyWithRoot" null null))

(fn `UserConstructionScript`
  (`parent.UserConstructionScript`))