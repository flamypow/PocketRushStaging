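; Projectile fired by the ground enemy that damages the player character on hit.
; On BeginPlay it looks up a BP_GroundEnemy through CharacterReference and copies that enemy's AttackDamage.
; On Hit it casts the other actor to BP_PocketRushCharacter_0020 and applies the stored damage.
; An unconnected cast to the older BP_PocketRushCharacter never runs, and the graph does not destroy the projectile.
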(event `self.ReceiveBeginPlay`
  ; Get Enemy Reference
  (bind _reference (`self.CharacterReference` "/Game/William/BP_GroundEnemy.BP_GroundEnemy_C"))
  (bind _asbp_ground_enemy (cast `/Game/William/BP_GroundEnemy` _reference))
  (bind _output_get (set `self.ShootEnemyRef` _asbp_ground_enemy))
  (set `self.AttackDamage` (`/Game/RobinStaging/Enemies/Characters/BP_BaseEnemy.AttackDamage` _output_get)))

(event `self.ReceiveHit`
  (params (MyComp :type "PrimitiveComponent Object Reference") (Other :type "Actor Object Reference") (OtherComp :type "PrimitiveComponent Object Reference") (bSelfMoved :type Boolean) (HitLocation :type "Vector Structure") (HitNormal :type "Vector Structure") (NormalImpulse :type "Vector Structure") (Hit :type "HitResult Structure (by ref)"))
  ; When hit the player
  (bind _asbp_pocket_rush_character_0020 (cast `/Game/Killian_Core/KillianContent/BP_PocketRushCharacter_0020` Other))
  (`self.DamageActor` _asbp_pocket_rush_character_0020 (`self.AttackDamage`)))

(fn `UserConstructionScript`
  (`parent.UserConstructionScript`))