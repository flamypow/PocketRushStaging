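; Gun component that gives the player a glide ability, triggered by IA_Ability while the gun is active.
; It stores the camera rotation, launches the character upward, then lowers gravity after a short delay.
; A counted, delay-driven event loop applies repeated forward and slightly upward impulses along that stored rotation.
; When the loop ends, it restores normal gravity and reduces charges.
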(event `EnhancedInput|/Game/Killian_Core/FirstPerson/Input/Actions/IA_Ability`
  (params (ActionValue :type Boolean) (ElapsedSeconds :type "Float (double-precision)") (TriggeredSeconds :type "Float (double-precision)") (InputAction :type "InputAction Object Reference" :default "/Game/Killian_Core/FirstPerson/Input/Actions/IA_Ability.IA_Ability"))
  (:`Triggered`
    (if (`self.ActiveGun`)
      (bind _output_get (set `/Game/Killian_Core/KillianContent/BP_PocketRushCharacter_0020.GlideRotation` (`PlayerCameraManager.GetCameraRotation` (`GameplayStatics.GetPlayerCameraManager` 0)) (`self.PocketChar`)))
      (set `self.Looptimes` 10)
      (`Character.LaunchCharacter` (`self.PocketChar`) (0.0 0.0 1000.0) false false)
      (`KismetSystemLibrary.Delay` 0.5)
      (set `CharacterMovementComponent.GravityScale` 0.3 (`Character.CharacterMovement` (`self.PocketChar`)))
      (`self.Addthrust`)
      (`self.ThrustCount`))))

(event `Addthrust`
  ; Event to add force, needs to loop so small and contained
  (`CharacterMovementComponent.AddImpulse` (`Character.CharacterMovement` (`self.PocketChar`)) (`KismetMathLibrary.GreaterGreater_VectorRotator` (250.0 0.0 100.0) (stale `EnhancedInput|/Game/Killian_Core/FirstPerson/Input/Actions/IA_Ability` _output_get)) true))

(event `ThrustCount`
  (bind _result (`/Engine/EditorBlueprintResources/StandardMacros.DecrementInt` (`self.Looptimes`))
    (:`  `
      (`KismetSystemLibrary.Delay` 0.02)
      (if (> _result 0)
        (`self.Addthrust`)
        (`self.ThrustCount`)
        (else
          (set `CharacterMovementComponent.GravityScale` 1.0 (`Character.CharacterMovement` (`self.PocketChar`)))
          (`self.ReduceCharges`))))))