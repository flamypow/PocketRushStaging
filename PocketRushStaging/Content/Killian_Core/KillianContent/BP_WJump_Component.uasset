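; BP_WJump_Component is a gun ability component that gives the player a charge-based vertical jump.
; On the IA_Ability input, it requires ActiveGun and a valid first child component on PocketChar's first-person mesh.
; It zeroes vertical velocity before launching the character upward, keeping horizontal momentum and a consistent boost, then calls ReduceCharges.
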(event `EnhancedInput|/Game/Killian_Core/FirstPerson/Input/Actions/IA_Ability`
  (params (ActionValue :type Boolean) (ElapsedSeconds :type "Float (double-precision)") (TriggeredSeconds :type "Float (double-precision)") (InputAction :type "InputAction Object Reference" :default "/Game/Killian_Core/FirstPerson/Input/Actions/IA_Ability.IA_Ability"))
  (bind _pocketchar (`self.PocketChar`))
  (bind _charactermovement (`Character.CharacterMovement` _pocketchar))
  (bind (_velocity_x _velocity_y) (`KismetMathLibrary.BreakVector` (`MovementComponent.Velocity` _charactermovement)))
  (:`Triggered`
    (if (`self.ActiveGun`)
      (`/Engine/EditorBlueprintResources/StandardMacros.IsValid` (`self.GetChildComponent` (`/Game/Killian_Core/KillianContent/BP_PocketRushCharacter_0020.FirstPersonMesh` _pocketchar) 0)
        (:`Is Valid`
          (set `MovementComponent.Velocity` (`KismetMathLibrary.MakeVector` _velocity_x _velocity_y) _charactermovement)
          (`Character.LaunchCharacter` _pocketchar (0.0 0.0 1000.0) false false)
          (`self.ReduceCharges`))))))