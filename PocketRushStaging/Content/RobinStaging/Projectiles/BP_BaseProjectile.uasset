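; BP_BaseProjectile is a base projectile actor that deals damage scaled to a character's attack stat.
; On BeginPlay it caches the first actor of CharClassRef found in the level as CharObjRef.
; DamageActor applies that character's AttackDamage to a given actor, though nothing in this Blueprint calls it.
; The projectile destroys itself when its ProjectileMovement component stops.
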(event `self.ReceiveBeginPlay`
  ; Create Reference
  (bind _outactors (`GameplayStatics.GetAllActorsOfClass` (`self.CharClassRef`)))
  (set `self.CharObjRef` (`|GetArrayItem` _outactors)))

(event `self.ProjectileMovement.OnProjectileStop`
  (params (ImpactResult :type "HitResult Structure (by ref)"))
  ; When the projectile stops moving
  (`self.K2_DestroyActor`))

(fn `DamageActor`
  (params (DamagedActor :type "Actor Object Reference"))
  (`GameplayStatics.ApplyDamage` DamagedActor (`KismetMathLibrary.Conv_IntToDouble` (`/Game/RobinStaging/Characters/BP_BaseCharacter.AttackDamage` (`self.CharObjRef`)))))

(fn `UserConstructionScript`)