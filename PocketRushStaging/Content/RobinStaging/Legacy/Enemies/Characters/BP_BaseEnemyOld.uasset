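; BP_BaseEnemyOld is a legacy base enemy that handles health, death and an overhead health bar.
; It starts at full HP, subtracts incoming AnyDamage and destroys itself when health runs out.
; Every tick, the widget bar updates its fill, rotates toward the player camera and hides at full health.
; CheckPlayer smoothly yaws the enemy toward a BP_Player_Old, but nothing in this Blueprint calls it.
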(event `self.ReceiveBeginPlay`
  ; Initialize Current Health
  (set `self.CurrentHealth` (`self.HP`)))

(event `self.ReceiveAnyDamage`
  (params (Damage :type "Float (single-precision)") (DamageType :type "DamageType Object Reference") (InstigatedBy :type "Controller Object Reference") (DamageCauser :type "Actor Object Reference"))
  ; Damage Taken
  (`self.DamageTaken` Damage))

(event `self.ReceiveTick`
  (params (DeltaSeconds :type "Float (single-precision)"))
  ; Enemy HP UI
  (`self.EnemyHPUI`))

(fn `CheckPlayer`
  (params (PlayerObj :type "Object Object Reference"))
  (bind _asbp_player_old (cast `/Game/RobinStaging/Legacy/FirstPerson/Blueprints/BP_Player_Old` PlayerObj))
  (bind (_returnvalue_roll _returnvalue_pitch _returnvalue_yaw) (`KismetMathLibrary.BreakRotator` (`KismetMathLibrary.RInterpTo` (`self.K2_GetActorRotation`) (`KismetMathLibrary.FindLookAtRotation` (`self.K2_GetActorLocation`) (`self.K2_GetActorLocation` _asbp_player_old)) (`GameplayStatics.GetWorldDeltaSeconds`) (`self.LookSpeed`))))
  (`self.K2_SetActorRotation` (`KismetMathLibrary.MakeRotator` 0.0 0.0 _returnvalue_yaw)))

(fn `DamageTaken`
  (params (ReceivedDamage :type "Float (double-precision)"))
  (bind _output_get (set `self.CurrentHealth` (- (`self.CurrentHealth`) ReceivedDamage)))
  (if (<= _output_get 0.0)
    (`self.K2_DestroyActor`)))

(fn `UserConstructionScript`)