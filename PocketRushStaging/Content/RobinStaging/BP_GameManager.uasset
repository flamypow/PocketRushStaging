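; Game manager Blueprint that handles pausing and switching between gameplay and menu modes, starting in game mode on BeginPlay.
; SwitchModeGameUI toggles the mouse cursor, input mode and game pause state together.
; PauseGame lazily creates and caches the pause menu widget, adding it to the viewport.
; Only later calls, with a valid cached widget, make it visible and switch to UI mode; the creation branch leaves the mode unchanged.
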(event `self.ReceiveBeginPlay`
  ; Set Game Mode
  (`self.SwitchMode(Game/UI)` false (`GameplayStatics.GetPlayerController` 0)))

(fn `PauseGame`
  (bind _pausemenuobjref (`self.PauseMenuObjRef`))
  (`/Engine/EditorBlueprintResources/StandardMacros.IsValid` _pausemenuobjref
    (:`Is Valid`
      (`Widget.SetVisibility` _pausemenuobjref "Visible")
      (`self.SwitchMode(Game/UI)` true (`GameplayStatics.GetPlayerController` 0)))
    (:`Is Not Valid`
      (bind _returnvalue (`|CreateWidget` (`self.PauseMenuClassRef`)))
      (bind _output_get (set `self.PauseMenuObjRef` _returnvalue))
      (`UserWidget.AddToViewport` _output_get 0))))

(fn `SwitchMode(Game/UI)`
  (params (`Is Menu Mode` :type Boolean) (`Player Controller` :type "PlayerController Object Reference"))
  (set `PlayerController.bShowMouseCursor` `Is Menu Mode` `Player Controller`)
  (if `Is Menu Mode`
    (`WidgetBlueprintLibrary.SetInputMode_UIOnlyEx` `Player Controller` null)
    (`GameplayStatics.SetGamePaused` true)
    (else
      (`WidgetBlueprintLibrary.SetInputMode_GameOnly` `Player Controller`)
      (`GameplayStatics.SetGamePaused` false))))

(fn `UserConstructionScript`)